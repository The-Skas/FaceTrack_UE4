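; Sandbox character Blueprint for experimenting with webcam face tracking over OSC and morph-target facial animation.
; The first OSC receiver matches found, position and orientation addresses but stores only zeros, printing on both pose messages.
; Float parsing and bone-posing nodes are disconnected, and the second receiver is empty.
; Input is enabled on BeginPlay, and B prints a debug string and fully raises the left-brow morph on the Mesh.
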(event Custom|OnOscReceived_OscReceiver1_Copy_1
  (params (Address :type Name%20%28by%20ref%29) (Data :type Osc%20Data%20Struct%20Structure%20%28by%20ref%29))
  ;[1 1 1] Deal with income OSC messages from webcam.
)

(event Custom|OnOscReceived_OscReceiver1_Copy
  (params (Address :type Name%20%28by%20ref%29) (Data :type Osc%20Data%20Struct%20Structure%20%28by%20ref%29))
  (bind _returnvalue (Math|Vector|MakeVector 0.0 0.0 0.0))
  ;[1 1 1] Deal with income OSC messages from webcam.
  (Utilities|FlowControl|Sequence
    (:then_0
      (switch name Address
        (:/found
          (Variables|Default|Setfound 0.0))
        (:/pose/position
          (Variables|Default|SetPosition _returnvalue)
          (Development|PrintString "Hello" :!label _label))
        (:/pose/orientation
          (Variables|Default|SetOrientation _returnvalue)
          (goto _label))))))

(event EventTick
  (params (DeltaSeconds :type Float%20%28single-precision%29)))

(event EventBeginPlay
  ;[1 1 1] Sandbox
  (Input|EnableInput (Game|GetPlayerController 0)))

(event Input|KeyboardEvents|B
  ;[1 1 1] Sandbox
  (:Pressed
    (Development|PrintString "Hero:" true true "(R=1.000000,G=0.000000,B=0.366009,A=1.000000)")
    (Components|SkeletalMesh|SetMorphTarget (Variables|Character|GetMesh) "BrowsUp_Left" 1.0)))

(fn ConstructionScript)