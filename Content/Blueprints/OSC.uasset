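; Blueprint that receives face-tracking data over OSC and exposes it as face events.
; OscReceiver1 routes messages by address to events for found state, position, orientation, scale and expression, all empty here.
; PopNTimes pops floats from the message into a vector, and orientation swaps its X and Z components.
; Expression is read as a string, and the PopN loop is an unfinished stub.
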(event OnOscReceived(OscReceiver1)
  (params (Address :type Name%20%28by%20ref%29 :default "None") (Data :type Osc%20Data%20Struct%20Structure%20%28by%20ref%29))
  (switch name Address
    (:/found
      (bind _result (CallFunction|PopNTimes 1 Data))
      ;[1 1 1] Event Callers
      (CallFunction|FaceFound (== (.X (Math|Vector|BreakVector _result)) 1.0)))
    (:/pose/position
      (bind _result_2 (CallFunction|PopNTimes 3 Data))
      (CallFunction|FacePosition _result_2))
    (:/pose/orientation
      (bind _result_3 (CallFunction|PopNTimes 3 Data))
      (CallFunction|FaceOrientation (Math|Vector|MakeVector (.Z (Math|Vector|BreakVector _result_3)) (.Y (Math|Vector|BreakVector _result_3)) (.X (Math|Vector|BreakVector _result_3)))))
    (:/pose/scale
      (bind _result_4 (CallFunction|PopNTimes 1 Data))
      (CallFunction|FaceScale (.X (Math|Vector|BreakVector _result_4))))
    (:/expression
      (CallFunction|FaceExpression (.Value (Class|OscFunctionLibrary|PopString Data))))))

(event Custom|Face%20Scale
  (params (Facial%20Scale :type Float%20%28single-precision%29))
  ;[1 1 1] Events
)

(event Custom|Face%20Position
  (params (FacePosition :type Vector))
  ;[1 1 1] Events
)

(event Custom|Face%20Found
  (params (isFaceFound :type Boolean))
  ;[1 1 1] Events
)

(event Custom|Face%20Expression
  (params (FacialExpression :type Name :default "neutral"))
  ;[1 1 1] Events
)

(event Custom|Face%20Orientation
  (params (Face%20Orientation :type Vector))
  ;[1 1 1] Events
)

(fn ConstructionScript)

(fn PopNTimes
  (params (N_TIMES :type Integer) (Data :type Osc%20Data%20Struct%20Structure))
  (bind _array_data (LocalVariables|Getarray_data))
  (LocalVariables|SetTempDataStruc Data)
  (for _index (range 1 N_TIMES)
    (Utilities|Array|Add (LocalVariables|Getarray_data) (.Value (Class|OscFunctionLibrary|PopFloat (LocalVariables|GetTempDataStruc))))
    (LocalVariables|SetTempDataStruc (.output (Class|OscFunctionLibrary|PopFloat (LocalVariables|GetTempDataStruc)))))
  (return (Math|Vector|MakeVector (Utilities|Array|Get(acopy) _array_data) (Utilities|Array|Get(acopy) _array_data 1) (Utilities|Array|Get(acopy) _array_data 2))))