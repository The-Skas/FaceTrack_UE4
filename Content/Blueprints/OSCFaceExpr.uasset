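; OSCFaceExpr applies incoming facial expressions, labelled as coming from Python, to a mesh through morph targets.
; The FaceExpression event stores the received expression, searches the Expressions array for matches, and sets each matching entry's morph target values on Mymesh.
; Every comparison prints a debug string showing the Python and Unreal values, while FaceFound and Tick have no effect.
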(event EventFaceFound
  (params (isFaceFound :type Boolean))
  (if (Math|Boolean|NotEqual(Boolean) isFaceFound true)
    _))

(event EventFaceExpression
  (params (FacialExpression :type Name :default "None"))
  (Variables|Default|Setexpression FacialExpression)
  (for _array_element (Variables|Default|Getexpressions)
    (Development|PrintString (Utilities|String|ToString(Text) (Utilities|Text|FormatText "Python - {python} - Unreal - {ue}" (Utilities|Text|ToText(String) (Utilities|String|ToString(Name) (Variables|Default|Getexpression))) (Utilities|Text|ToText(Name) (.expression (Utilities|Struct|BreakStructFacialExpressions _array_element))))))
    (if (Utilities|Name|Equal(Name) (Variables|Default|Getexpression) (.expression (Utilities|Struct|BreakStructFacialExpressions _array_element)))
      (for _array_element_2 (.morphTargets (Utilities|Struct|BreakStructFacialExpressions _array_element))
        (Components|SkeletalMesh|SetMorphTarget (Variables|Default|Getmymesh) (.MorphTarget (Utilities|Struct|BreakStructMorphTarget _array_element_2)) (.Value (Utilities|Struct|BreakStructMorphTarget _array_element_2)))))))

(event EventTick
  (params (DeltaSeconds :type Float%20%28single-precision%29)))

(fn ConstructionScript
  (|CallParentFunction))